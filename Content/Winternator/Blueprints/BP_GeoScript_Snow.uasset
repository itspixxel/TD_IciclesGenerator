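; Geometry Script generated mesh actor that builds a snow layer over the static mesh actors in ActorsToProcess.
; On rebuild, Process skips oversized actors, copies each mesh in world space, keeps upward-facing triangles, extrudes and offsets them by SnowThickness, then appends the result.
; The combined mesh gets uniform remeshing, Perlin noise, smoothing, recomputed normals and XAtlas UVs.
; An unconnected line-trace box and sphere experiment remains in the graph.
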(event Events|EventOnRebuildGeneratedMesh
  (params (TargetMesh :type Dynamic%20Mesh%20Object%20Reference))
  (CallFunction|Process TargetMesh))

(fn ConstructionScript)

(fn Process
  (params (DynaMesh :type Dynamic%20Mesh%20Object%20Reference))
  (for _array_element (Variables|SnowyActors|GetActorsToProcess)
    (if (< (Math|Vector|VectorLength (.BoxExtent (Collision|GetComponentBounds (Variables|/Script/Engine.StaticMeshActor|GetStaticMeshComponent _array_element)))) (Variables|SnowSettings|GetReject%20Actors%20Bigger%20Than))
      (Utilities|FlowControl|Sequence
        (:then_0
          ;[0.01764 0.01764 0.01764] Allocate temp dyna mesh to work on
          (bind _returnvalue (DynamicMeshActor|AllocateComputeMesh))
          (LocalVariables|SetCurrDynaMesh _returnvalue))
        (:then_1
          ;[0.01764 0.01764 0.01764] Copy geometry from static mesh actor in world space
          (bind _returnvalue_2 (GeometryScript|StaticMesh|CopyMeshFromStaticMesh :FromStaticMeshAsset (Variables|/Script/Engine.StaticMeshComponent|GetStaticMesh (Variables|/Script/Engine.StaticMeshActor|GetStaticMeshComponent _array_element)) :ToDynamicMesh (LocalVariables|GetCurrDynaMesh) :Debug 0)
            (:Failure
              _)
            (:Success
              _))
          (GeometryScript|Transforms|TransformMesh _returnvalue_2 (Transformation|GetWorldTransform (Variables|/Script/Engine.StaticMeshActor|GetStaticMeshComponent _array_element)) true 0))
        (:then_2
          ;[0.01764 0.01764 0.01764] Select triangles that don't point upwards and delete them
          (bind _selection (Class|GeometryScriptLibraryMeshSelectionFunctions|SelectMeshElementsbyNormalAngle (LocalVariables|GetCurrDynaMesh) "0.000000,0.000000,1.000000" 8e+01 "Triangles" true))
          (LocalVariables|SetCurrSelectedTris _selection))
        (:then_3
          (Class|GeometryScriptLibraryMeshBasicEditFunctions|DeleteSelectedTrianglesfromMesh (LocalVariables|GetCurrDynaMesh) (LocalVariables|GetCurrSelectedTris) false))
        (:then_4
          ;[0.01764 0.01764 0.01764] Extrude remaining geometry upwards and inflate it
          (bind _returnvalue_3 (Class|GeometryScriptLibraryMeshModelingFunctions|ApplyMeshLinearExtrudeFaces :TargetMesh (LocalVariables|GetCurrDynaMesh) :Options (Utilities|Struct|MakeGeometryScriptMeshLinearExtrudeOptions (Variables|SnowSettings|GetSnow%20Thickness) "AverageFaceNormal" "0.000000,0.000000,1.000000" "EntireSelection" "(GroupMode=PreserveExisting,ConstantGroup=0)" 1.0 true) :Debug 0))
          (Class|GeometryScriptLibraryMeshModelingFunctions|ApplyMeshOffset _returnvalue_3 (Utilities|Struct|MakeGeometryScriptMeshOffsetOptions (Variables|SnowSettings|GetSnow%20Thickness) false 5 0.1 false 0.2) 0))
        (:then_5
          ;[0.01764 0.01764 0.01764] Append result to main dyna mesh
          (GeometryScript|MeshEdits|AppendMesh DynaMesh (LocalVariables|GetCurrDynaMesh) (Math|Transform|InvertTransform (Transformation|GetWorldTransform (Variables|DynamicMeshActor|GetDynamicMeshComponent))) false "(CombineMode=EnableAllMatching)" 0)))))
  ;[0.01764 0.01764 0.01764] Apply post processes to the final result
  (bind _returnvalue_4 (Class|GeometryScriptLibraryRemeshingFunctions|ApplyUniformRemesh DynaMesh (Utilities|Struct|MakeGeometryScriptRemeshOptions true "Uniform" (Variables|SnowSettings|GetRemesh%20Iterations)) (Utilities|Struct|MakeGeometryScriptUniformRemeshOptions (Variables|SnowSettings|GetRemesh%20Type) (Variables|SnowSettings|GetRemesh%20Target%20Triangle%20Count) (Variables|SnowSettings|GetRemesh%20Target%20Edge%20Length)) 0))
  (bind _returnvalue_5 (Class|GeometryScriptLibraryMeshDeformFunctions|ApplyPerlinNoisetoMesh :TargetMesh _returnvalue_4 :Options (Utilities|Struct|MakeGeometryScriptPerlinNoiseOptions (Utilities|Struct|MakeGeometryScriptPerlinNoiseLayerOptions (Variables|SnowSettings|GetPerlin%20Noise%20Magnitude) (Variables|SnowSettings|GetPerlin%20Noise%20Frequency) "0.000000,0.000000,0.000000" (Variables|SnowSettings|GetPerlin%20Noise%20Seed)) true "FullMeshSelection") :Debug 0))
  (bind _returnvalue_6 (Class|GeometryScriptLibraryMeshDeformFunctions|ApplyIterativeSmoothingtoMesh :TargetMesh _returnvalue_5 :Options (Utilities|Struct|MakeGeometryScriptIterativeMeshSmoothingOptions 6 0.1 "FullMeshSelection") :Debug 0))
  (bind _returnvalue_7 (GeometryScript|Normals|RecomputeNormals :TargetMesh _returnvalue_6 :Debug 0))
  (Class|GeometryScriptLibraryMeshUVFunctions|AutoGenerateXAtlasMeshUVs :TargetMesh _returnvalue_7 :Debug 0))