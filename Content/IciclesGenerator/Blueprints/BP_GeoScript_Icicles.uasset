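; Geometry Script generated-mesh actor that procedurally grows icicles under a sampled static mesh actor, within a sphere around itself.
; On rebuild it selects downward-facing triangles in that sphere, offsets them and simplifies to a target vertex count, using the vertices as scatter points.
; Seeded random cones are appended there, then noised, solidified, decimated and given new normals.
; Only the icicle mesh replaces the output.
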(event Events|EventOnRebuildGeneratedMesh
  (params (TargetMesh :type Dynamic%20Mesh%20Object%20Reference))
  (CallFunction|Process TargetMesh))

(fn ConstructionScript)

(fn Process
  (params (DynaMesh :type Dynamic%20Mesh%20Object%20Reference))
  (bind _cone_radius (Variables|IciclesSettings|GetCone%20Radius))
  (bind _cone_height (Variables|IciclesSettings|GetCone%20Height))
  (Components|Sphere|SetSphereRadius (Variables|Components|GetRadius%20Visualizer) (Variables|IciclesSettings|GetSphere%20Radius) true)
  (bind _returnvalue (DynamicMesh|Reset DynaMesh))
  (Utilities|FlowControl|Sequence
    (:then_0
      ;[0.01764 0.01764 0.01764] Allocate temp dyna mesh to work on
      (bind _returnvalue_2 (DynamicMeshActor|AllocateComputeMesh))
      (Variables|Default|SetTempDynamicMesh _returnvalue_2))
    (:then_1
      ;[0.01764 0.01764 0.01764] Initialize a deterministic RNG
      (Variables|Default|SetRandom%20Stream (Math|Random|MakeRandomStream (Variables|IciclesSettings|GetRandom%20Seed))))
    (:then_2
      ;[0.01764 0.01764 0.01764] Save the transforms for later
      (Variables|Default|SetSelf%20Location%20World (Transformation|GetWorldLocation (Variables|DynamicMeshActor|GetDynamicMeshComponent)))
      (Variables|Default|SetSelf%20Transform%20World%20Inverted (Math|Transform|InvertTransform (Transformation|GetWorldTransform (Variables|DynamicMeshActor|GetDynamicMeshComponent)))))
    (:then_3
      ;[0.01764 0.01764 0.01764] Copy the geometry from the static mesh
      (bind _localtoworld (GeometryScript|Scene|CopyMeshfromComponent :Component (Variables|/Script/Engine.StaticMeshActor|GetStaticMeshComponent (Variables|IciclesSettings|GetActor%20to%20Sample)) :ToDynamicMesh (Variables|Default|GetTempDynamicMesh) :bTransformToWorld true :Debug 0)
        (:Failure
          _)
        (:Success
          _))
      (Variables|Default|SetMeshSourceLocalToWorld _localtoworld))
    (:then_4
      ;[0.01764 0.01764 0.01764] Make a selection of downwards facing triangles within defined sphere
      (bind _selection (Class|GeometryScriptLibraryMeshSelectionFunctions|SelectMeshElementsbyNormalAngle (Variables|Default|GetTempDynamicMesh) "0.000000,0.000000,-1.000000" 4e+01 "Triangles" false))
      (bind _selection_2 (Class|GeometryScriptLibraryMeshSelectionFunctions|SelectMeshElementsinSphere (Variables|Default|GetTempDynamicMesh) (Variables|Default|GetSelf%20Location%20World) (Variables|IciclesSettings|GetSphere%20Radius) "Triangles" false))
      (bind _resultselection (Class|GeometryScriptLibraryMeshSelectionFunctions|CombineMeshSelections _selection _selection_2 "Intersection"))
      (LocalVariables|SetTrianglesFacingDown _resultselection))
    (:then_5
      ;[0.01764 0.01764 0.01764] Copy only the selected tris into the mesh
      (bind _storetosubmeshout (Class|GeometryScriptLibraryMeshDecompositionFunctions|CopyMeshSelectiontoMesh (Variables|Default|GetTempDynamicMesh) _returnvalue (LocalVariables|GetTrianglesFacingDown) false false 0))
      (GeometryScript|Transforms|TransformMesh _storetosubmeshout (Variables|Default|GetSelf%20Transform%20World%20Inverted) true 0))
    (:then_6
      ;[0.01764 0.01764 0.01764] Make mesh thicker
      (Class|GeometryScriptLibraryMeshModelingFunctions|ApplyMeshOffset _returnvalue (Utilities|Struct|MakeGeometryScriptMeshOffsetOptions (Variables|IciclesSettings|GetExtrusion%20Bias) false 3 0.1 false 0.2) 0))
    (:then_7
      ;[0.01764 0.01764 0.01764] Scatter points on the mesh for icicles
      (bind _returnvalue_3 (GeometryScript|Simplification|ApplySimplifytoVertexCount _returnvalue (Variables|IciclesSettings|GetPoints%20To%20Scatter) (Utilities|Struct|MakeGeometryScriptSimplifyMeshOptions "VolumePreserving" true true true false false true) 0))
      (bind _positionlist (GeometryScript|MeshQueries|GetAllVertexPositions _returnvalue_3))
      (bind _vectorarray (Class|GeometryScriptLibraryListUtilityFunctions|ConvertVectorListtoArray _positionlist))
      ;[0.01764 0.01764 0.01764] Append cones at scattered points
      (DynamicMesh|Reset (Variables|Default|GetTempDynamicMesh))
      (for _array_element _vectorarray
        (bind _output_get (Variables|Default|SetCone%20Radius%20Current (Math|Random|RandomFloatinRangefromStream (Variables|Default|GetRandom%20Stream) (* _cone_radius 0.2) _cone_radius)))
        (Class|GeometryScriptLibraryMeshPrimitiveFunctions|AppendCone :TargetMesh (Variables|Default|GetTempDynamicMesh) :Transform (Math|Transform|MakeTransform _array_element "180.000000,0.000000,0.000000") :BaseRadius (Math|Random|RandomFloatinRangefromStream (Variables|Default|GetRandom%20Stream) (* _cone_radius 0.2) _cone_radius) :TopRadius (* _output_get 0.1) :Height (Math|Random|RandomFloatinRangefromStream (Variables|Default|GetRandom%20Stream) (* _cone_height 0.3) _cone_height) :RadialSteps 24 :HeightSteps 24 :Debug 0)))
    (:then_8
      ;[0.01764 0.01764 0.01764] Apply post processes to icicles
      (bind _returnvalue_4 (Class|GeometryScriptLibraryMeshDeformFunctions|ApplyPerlinNoisetoMesh :TargetMesh (Variables|Default|GetTempDynamicMesh) :Options (Utilities|Struct|MakeGeometryScriptPerlinNoiseOptions (Utilities|Struct|MakeGeometryScriptPerlinNoiseLayerOptions (* (Variables|IciclesSettings|GetCone%20Radius) 0.15) 0.25 "0.000000,0.000000,0.000000" 0) true "FullMeshSelection") :Debug 0))
      (bind _returnvalue_5 (Class|GeometryScriptLibraryMeshVoxelFunctions|ApplyMeshSolidify _returnvalue_4 (Utilities|Struct|MakeGeometryScriptSolidifyOptions (Utilities|Struct|MakeGeometryScript3DGridParameters "GridResolution" 0.5 96) 0.5 true 1.0 3 false 1.0) 0))
      (bind _returnvalue_6 (Class|GeometryScriptLibraryMeshSimplifyFunctions|ApplySimplifytoTolerance _returnvalue_5 (Variables|IciclesSettings|GetDecimation%20Tolerance) (Utilities|Struct|MakeGeometryScriptSimplifyMeshOptions "VolumePreserving" true true true false false true) 0))
      (GeometryScript|Normals|RecomputeNormals :TargetMesh _returnvalue_6 :Debug 0))
    (:then_9
      (bind _returnvalue_7 (DynamicMesh|Reset _returnvalue))
      (GeometryScript|Decomposition|CopyMeshtoMesh (Variables|Default|GetTempDynamicMesh) _returnvalue_7 0))))