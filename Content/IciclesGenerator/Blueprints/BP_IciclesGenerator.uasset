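; Generated dynamic mesh actor that uses Geometry Script to build a noisy shell, presumably ice, over listed static mesh actors.
; On rebuild, Process copies each mesh in world space, culls triangles by normal angle, then extrudes, offsets and appends the rest in local space.
; The merged result is uniformly remeshed, displaced with Perlin noise and smoothed.
; An unconnected line-trace experiment remains in the event graph.
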(event Events|EventOnRebuildGeneratedMesh
  (params (TargetMesh :type Dynamic%20Mesh%20Object%20Reference))
  (CallFunction|Process TargetMesh))

(fn ConstructionScript)

(fn Process
  (params (DynaMesh :type Dynamic%20Mesh%20Object%20Reference))
  (for _array_element (Variables|Default|GetActorsToProcess)
    (Utilities|FlowControl|Sequence
      (:then_0
        (bind _returnvalue (DynamicMeshActor|AllocateComputeMesh))
        (LocalVariables|SetCurrDynaMesh _returnvalue))
      (:then_1
        (bind _returnvalue_2 (GeometryScript|StaticMesh|CopyMeshFromStaticMesh :FromStaticMeshAsset (Variables|/Script/Engine.StaticMeshComponent|GetStaticMesh (Variables|/Script/Engine.StaticMeshActor|GetStaticMeshComponent _array_element)) :ToDynamicMesh (LocalVariables|GetCurrDynaMesh) :Debug 0)
          (:Failure
            _)
          (:Success
            _))
        (GeometryScript|Transforms|TransformMesh _returnvalue_2 (Transformation|GetWorldTransform (Variables|/Script/Engine.StaticMeshActor|GetStaticMeshComponent _array_element)) true 0))
      (:then_2
        (bind _selection (Class|GeometryScriptLibraryMeshSelectionFunctions|SelectMeshElementsbyNormalAngle (LocalVariables|GetCurrDynaMesh) "0.000000,0.000000,1.000000" 8e+01 "Triangles" true))
        (LocalVariables|SetCurrSelectedTris _selection))
      (:then_3
        (Class|GeometryScriptLibraryMeshBasicEditFunctions|DeleteSelectedTrianglesfromMesh (LocalVariables|GetCurrDynaMesh) (LocalVariables|GetCurrSelectedTris) false))
      (:then_4
        (bind _returnvalue_3 (Class|GeometryScriptLibraryMeshModelingFunctions|ApplyMeshLinearExtrudeFaces :TargetMesh (LocalVariables|GetCurrDynaMesh) :Options (Utilities|Struct|MakeGeometryScriptMeshLinearExtrudeOptions 5.0 "AverageFaceNormal" "0.000000,0.000000,1.000000" "EntireSelection" "(GroupMode=PreserveExisting,ConstantGroup=0)" 1.0 true) :Debug 0))
        (Class|GeometryScriptLibraryMeshModelingFunctions|ApplyMeshOffset _returnvalue_3 (Utilities|Struct|MakeGeometryScriptMeshOffsetOptions 5.0 false 5 0.1 false 0.2) 0))
      (:then_5
        (GeometryScript|MeshEdits|AppendMesh DynaMesh (LocalVariables|GetCurrDynaMesh) (Math|Transform|InvertTransform (Transformation|GetWorldTransform (Variables|DynamicMeshActor|GetDynamicMeshComponent))) false "(CombineMode=EnableAllMatching)" 0))))
  (bind _returnvalue_4 (Class|GeometryScriptLibraryRemeshingFunctions|ApplyUniformRemesh :TargetMesh DynaMesh :UniformOptions (Utilities|Struct|MakeGeometryScriptUniformRemeshOptions "TriangleCount" 30000 6.0) :Debug 0))
  (bind _returnvalue_5 (Class|GeometryScriptLibraryMeshDeformFunctions|ApplyPerlinNoisetoMesh :TargetMesh _returnvalue_4 :Options (Utilities|Struct|MakeGeometryScriptPerlinNoiseOptions (Utilities|Struct|MakeGeometryScriptPerlinNoiseLayerOptions 15.0 0.16 "0.000000,0.000000,0.000000" 0) true "FullMeshSelection") :Debug 0))
  (bind _returnvalue_6 (Class|GeometryScriptLibraryMeshDeformFunctions|ApplyIterativeSmoothingtoMesh :TargetMesh _returnvalue_5 :Options (Utilities|Struct|MakeGeometryScriptIterativeMeshSmoothingOptions 4 0.1 "FullMeshSelection") :Debug 0))
  (GeometryScript|Normals|RecomputeNormals :TargetMesh _returnvalue_6 :Debug 0))